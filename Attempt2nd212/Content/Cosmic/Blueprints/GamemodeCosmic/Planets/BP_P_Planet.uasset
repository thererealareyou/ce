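; Planet actor for the Cosmic Encounter mode, tinted by owner color and holding per-color ship counts, with Warp as a non-clickable special case.
; BeginPlay seeds hardcoded ships; UpdateShips respawns BP_P_Ship stacks, the first color centered and others ringed around it.
; Custom depth highlights candidates, while a Gate and Closed flag limit clicks, closing all planets after a pick.
; Picks and ship changes go through player controller 0.
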(event `self.ReceiveBeginPlay`
  (bind _shipstruct_amount_of_ships (break `/Game/Cosmic/Blueprints/GamemodeCosmic/Structures/AmountOfShips` (`self.ShipStruct`)))
  (bind _shipstruct_amount_of_ships_2 (break `/Game/Cosmic/Blueprints/GamemodeCosmic/Structures/AmountOfShips` (`self.ShipStruct`)))
  (bind _colorstruct_scolor (break `/Game/Cosmic/Blueprints/GamemodeCosmic/Structures/ColorStruct` (`self.ColorStruct`)))
  (bind _shipstruct_amount_of_ships_3 (break `/Game/Cosmic/Blueprints/GamemodeCosmic/Structures/AmountOfShips` (`self.ShipStruct`)))
  (bind _shipstruct_amount_of_ships_4 (break `/Game/Cosmic/Blueprints/GamemodeCosmic/Structures/AmountOfShips` (`self.ShipStruct`)))
  (bind _shipstruct_amount_of_ships_5 (break `/Game/Cosmic/Blueprints/GamemodeCosmic/Structures/AmountOfShips` (`self.ShipStruct`)))
  (`MeshComponent.SetVectorParameterValueOnMaterials` (`self.Mesh_Planet`) "Color" (`KismetMathLibrary.Conv_LinearColorToVector` (`KismetMathLibrary.Conv_ColorToLinearColor` (`BlueprintMapLibrary.Map_Find` _colorstruct_scolor (`self.Color`)))))
  (if (`KismetStringLibrary.EqualEqual_StrStr` (`self.Color`) "Warp")
    (`BlueprintMapLibrary.Map_Add` _shipstruct_amount_of_ships_2 "Красный" 6)
    (`BlueprintMapLibrary.Map_Add` _shipstruct_amount_of_ships_4 "Жёлтый" 10)
    (`self.Update Ships`)
    (else
      (`BlueprintMapLibrary.Map_Add` _shipstruct_amount_of_ships (`self.Color`) 4)
      (`BlueprintMapLibrary.Map_Add` _shipstruct_amount_of_ships_3 "Жёлтый" 2)
      (`BlueprintMapLibrary.Map_Add` _shipstruct_amount_of_ships_5 "Голубой" 2)
      (`self.Update Ships`)
      (add `self.OnClicked` (delegate `Choose`)))))

(event `Choose`
  (params (TouchedActor :type "Actor Object Reference") (ButtonPressed :type "Key Structure" :default "None"))
  (if (not (`self.Closed`))
    (`/Engine/EditorBlueprintResources/StandardMacros.Gate` true :!label _label
      (:`Exit`
        (`self.ChoosePlanetToAttack`)
        (bind _outactors (`GameplayStatics.GetAllActorsOfClass` "BP_P_Planet_C"))
        (for _array_element _outactors
          (`/Game/Cosmic/Blueprints/GamemodeCosmic/Planets/BPI_IsThisPlanetYours.CloseGateP` _array_element true))))))

(event `/Game/Cosmic/Blueprints/GamemodeCosmic/Planets/BPI_IsThisPlanetYours.Is Yours`
  (params (Color :type String) (`Is Choosing Enemy Planet` :type Boolean))
  (bind _shipstruct_amount_of_ships (break `/Game/Cosmic/Blueprints/GamemodeCosmic/Structures/AmountOfShips` (`self.ShipStruct`)))
  (if `Is Choosing Enemy Planet`
    (`PrimitiveComponent.SetRenderCustomDepth` (`self.Mesh_Planet`) (or (== Color (`self.Color`)) (and (`KismetStringLibrary.EqualEqual_StrStr` Color "*") (`KismetStringLibrary.NotEqual_StrStr` Color "Warp"))))
    (else
      (`PrimitiveComponent.SetRenderCustomDepth` (`self.Mesh_Planet`) (or (== Color (`self.Color`)) (!= (`BlueprintMapLibrary.Map_Find` _shipstruct_amount_of_ships Color) 0))))))

(event `/Game/Cosmic/Blueprints/GamemodeCosmic/Planets/BPI_IsThisPlanetYours.ChoosePlanet`
  (params (Color :type String) (IsJoker :type Boolean))
  (set `self.Closed` false)
  (if IsJoker
    (goto _label :!via `Open`)
    (elif (`KismetStringLibrary.EqualEqual_StrStr` Color (`self.Color`))
      (goto _label :!via `Open`)
      (else
        (goto _label :!via `Close`)))))

(event `/Game/Cosmic/Blueprints/GamemodeCosmic/Planets/BPI_IsThisPlanetYours.CloseGateP`
  (params (`Is Closed` :type Boolean))
  (set `self.Closed` `Is Closed`))

(fn `ChangeShips`
  (params (Color :type String) (Amount :type Integer) (IsFromWarp :type Boolean))
  (bind _asbp_pc_cosmic_encounter (cast `/Game/Cosmic/Blueprints/GamemodeCosmic/BP_PC_CosmicEncounter` (`GameplayStatics.GetPlayerController` 0)))
  (`/Game/Cosmic/Blueprints/GamemodeCosmic/BP_PC_CosmicEncounter.SR_Change_Ship_Struct` _asbp_pc_cosmic_encounter self Color Amount IsFromWarp))

(fn `ChoosePlanetToAttack`
  (bind _asbp_pc_cosmic_encounter (cast `/Game/Cosmic/Blueprints/GamemodeCosmic/BP_PC_CosmicEncounter` (`GameplayStatics.GetPlayerController` 0)))
  (`/Game/Cosmic/Blueprints/GamemodeCosmic/BP_PC_CosmicEncounter.OC_SendChoosedPlanet` _asbp_pc_cosmic_encounter self))

(fn `GetAmountOfShips`
  (returns (NewParam :type Integer))
  (locals (`Amount Of Ships` :type Integer))
  (bind _shipstruct_amount_of_ships (break `/Game/Cosmic/Blueprints/GamemodeCosmic/Structures/AmountOfShips` (`self.ShipStruct`)))
  (bind _values (`BlueprintMapLibrary.Map_Values` _shipstruct_amount_of_ships))
  (for _array_element _values
    (set `local.Amount Of Ships` (+ _array_element (`local.Amount Of Ships`))))
  (return (`local.Amount Of Ships`)))

(fn `GetPlayersOnThisPlanet`
  (returns (`Players On This Planet` :type "Array of String"))
  (locals (PlayersOnThisPlanet :type "Array of String"))
  (bind _shipstruct_amount_of_ships (break `/Game/Cosmic/Blueprints/GamemodeCosmic/Structures/AmountOfShips` (`self.ShipStruct`)))
  (bind _shipstruct_amount_of_ships_2 (break `/Game/Cosmic/Blueprints/GamemodeCosmic/Structures/AmountOfShips` (`self.ShipStruct`)))
  (bind _keys (`BlueprintMapLibrary.Map_Keys` _shipstruct_amount_of_ships_2))
  (for _array_element _keys
    (if (> (`BlueprintMapLibrary.Map_Find` _shipstruct_amount_of_ships _array_element) 0)
      (`KismetArrayLibrary.Array_Add` (`local.PlayersOnThisPlanet`) _array_element)))
  (return (`local.PlayersOnThisPlanet`)))

(fn `GetPositionOfShips`
  (params (`Index Of Color` :type Integer) (`Index Of Ship` :type Integer) (Max :type Integer) (`Planet Position` :type "Transform Structure"))
  (returns (Transform :type "Transform Structure"))
  (bind _planet_position (`local.Planet Position`))
  (bind _returnvalue (* 2.0 (`KismetMathLibrary.MultiplyByPi` (/ (`KismetMathLibrary.Conv_IntToDouble` `Index Of Color`) (`KismetMathLibrary.Conv_IntToDouble` (- Max 1))))))
  (if (== `Index Of Color` 0)
    (return (`KismetMathLibrary.MakeTransform` (`KismetMathLibrary.MakeVector` (.x (.location _planet_position)) (.y (.location _planet_position)) (`KismetMathLibrary.Conv_IntToDouble` (+ (* (`local.Index Of Ship`) 8) 7))) (struct) (1.5 1.5 1.0)))
    (else
      (return (`KismetMathLibrary.MakeTransform` (`KismetMathLibrary.MakeVector` (+ (.x (.location `Planet Position`)) (* (`KismetMathLibrary.Sin` _returnvalue) 30.0)) (+ (.y (.location `Planet Position`)) (* (`KismetMathLibrary.Cos` _returnvalue) 30.0)) (`KismetMathLibrary.Conv_IntToDouble` (+ (* `Index Of Ship` 8) 7))) (struct) (1.5 1.5 1.0))))))

(fn `Update Ships`
  (bind _players_on_this_planet (`self.GetPlayersOnThisPlanet`))
  (bind _shipstruct_amount_of_ships (break `/Game/Cosmic/Blueprints/GamemodeCosmic/Structures/AmountOfShips` (`self.ShipStruct`)))
  (bind _outactors (`GameplayStatics.GetAllActorsOfClass` "/Game/Cosmic/Blueprints/GamemodeCosmic/Planets/BP_P_Ship.BP_P_Ship_C"))
  (for _array_element _outactors
    (if (== self (`/Game/Cosmic/Blueprints/GamemodeCosmic/Planets/BP_P_Ship.Planet` _array_element))
      (`self.K2_DestroyActor` _array_element)))
  (for (_array_element_2 _array_index) _players_on_this_planet
    (for _index (range 1 (+ (`BlueprintMapLibrary.Map_Find` _shipstruct_amount_of_ships _array_element_2) 1))
      (bind _transform (`self.GetPositionOfShips` _array_index _index (`KismetArrayLibrary.Array_Length` _players_on_this_planet) (`self.GetTransform`)))
      (`|SpawnActorFromClass` "/Game/Cosmic/Blueprints/GamemodeCosmic/Planets/BP_P_Ship.BP_P_Ship_C" _transform "Undefined" "MultiplyWithRoot" null _array_element_2 self null))))

(fn `UserConstructionScript`
  (bind _colorstruct_scolor (break `/Game/Cosmic/Blueprints/GamemodeCosmic/Structures/ColorStruct` (`self.ColorStruct`)))
  (bind (_value _returnvalue) (`BlueprintMapLibrary.Map_Find` _colorstruct_scolor (`self.Color`)))
  (bind _returnvalue_2 (`PrimitiveComponent.CreateDynamicMaterialInstance` (`self.Mesh_Planet`) 0 "/Game/Cosmic/Blueprints/GamemodeCosmic/Materials/ColorMaterial.ColorMaterial" "None"))
  (if _returnvalue
    (`MaterialInstanceDynamic.SetVectorParameterValue` _returnvalue_2 "Color" (`KismetMathLibrary.Conv_ColorToLinearColor` _value))))