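; Clickable planet ship for the Cosmic game mode, tinted by its color key from a color lookup.
; Interface events highlight matching-color ships via custom depth and open a click gate when color matches, ships remain and the planet isn't Warp.
; A click through the open gate adds one ship to the planet, passing a from-warp flag, then tells all BPI_IsThisShipYours actors to recheck remaining ships and close their gates.
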(event `self.ReceiveBeginPlay`
  (bind _colorstruct_scolor (break `/Game/Cosmic/Blueprints/GamemodeCosmic/Structures/ColorStruct` (`self.ColorStruct`)))
  (`MeshComponent.SetVectorParameterValueOnMaterials` (`self.Mesh_Ship`) "Color" (`KismetMathLibrary.Conv_LinearColorToVector` (`KismetMathLibrary.Conv_ColorToLinearColor` (`BlueprintMapLibrary.Map_Find` _colorstruct_scolor (`self.Color`)))))
  (add `self.OnClicked` (delegate `Add`)))

(event `Add` :!signature `self.OnClicked`
  (params (TouchedActor :type "Actor Object Reference") (ButtonPressed :type "Key Structure" :default "None"))
  (if (not (`self.Closed`))
    (`/Engine/EditorBlueprintResources/StandardMacros.Gate` true :!label _label
      (:`Exit`
        (`/Game/Cosmic/Blueprints/GamemodeCosmic/Planets/BP_P_Planet.ChangeShips` (`self.Planet`) (stale `/Game/Cosmic/Blueprints/GamemodeCosmic/Planets/BPI_IsThisShipYours.AddShip` Color) 1 (stale `/Game/Cosmic/Blueprints/GamemodeCosmic/Planets/BPI_IsThisShipYours.AddShip` IsThisShipFromWarp))
        (bind _outactors (`GameplayStatics.GetAllActorsWithInterface` "/Game/Cosmic/Blueprints/GamemodeCosmic/Planets/BPI_IsThisShipYours.BPI_IsThisShipYours_C"))
        (for _array_element _outactors
          (message `/Game/Cosmic/Blueprints/GamemodeCosmic/Planets/BPI_IsThisShipYours.AnyMoreShips` _array_element (stale `/Game/Cosmic/Blueprints/GamemodeCosmic/Planets/BPI_IsThisShipYours.AddShip` Color))
          (message `/Game/Cosmic/Blueprints/GamemodeCosmic/Planets/BPI_IsThisShipYours.CloseGate` _array_element true))))))

(event `/Game/Cosmic/Blueprints/GamemodeCosmic/Planets/BPI_IsThisShipYours.IsYours`
  (params (Color :type String))
  (`PrimitiveComponent.SetRenderCustomDepth` (`self.Mesh_Ship`) (== Color (`self.Color`))))

(event `/Game/Cosmic/Blueprints/GamemodeCosmic/Planets/BPI_IsThisShipYours.AddShip`
  (params (Color :type String) (AreThereStillAny :type Boolean) (IsThisShipFromWarp :type Boolean))
  (set `self.Closed` false)
  (if (`KismetStringLibrary.NotEqual_StrStr` (`/Game/Cosmic/Blueprints/GamemodeCosmic/Planets/BP_P_Planet.Color` (`self.Planet`)) "Warp")
    (if (`KismetStringLibrary.EqualEqual_StrStr` Color (`self.Color`))
      (if AreThereStillAny
        (goto _label :!via `Open`)
        (else
          (goto _label :!via `Close`)))
      (else
        (goto _label :!via `Close`)))
    (else
      (goto _label :!via `Close`))))

(event `/Game/Cosmic/Blueprints/GamemodeCosmic/Planets/BPI_IsThisShipYours.CloseGate`
  (params (IsClosed :type Boolean))
  (set `self.Closed` IsClosed))

(fn `UserConstructionScript`
  (bind _colorstruct_scolor (break `/Game/Cosmic/Blueprints/GamemodeCosmic/Structures/ColorStruct` (`self.ColorStruct`)))
  (bind _returnvalue (`PrimitiveComponent.CreateDynamicMaterialInstance` (`self.Mesh_Ship`) 0 null "None"))
  (`MaterialInstanceDynamic.SetVectorParameterValue` _returnvalue "Color" (`KismetMathLibrary.Conv_ColorToLinearColor` (`BlueprintMapLibrary.Map_Find` _colorstruct_scolor (`self.Color`)))))