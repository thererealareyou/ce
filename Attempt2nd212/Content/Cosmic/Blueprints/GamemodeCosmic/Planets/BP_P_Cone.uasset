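; Attack cone for a Cosmic Encounter game, showing attacking and defending ships in an encounter at a planet.
; BeginPlay copies the defender's planet count, adds hard-coded colour counts, then calls UpdateShips on authority.
; UpdateShips respawns owned BP_P_Ship actors as per-colour stacks, placed on trigonometric arcs derived from planet count, with special spots for both main players.
; ChangeShips forwards count changes to the player controller's SRChangeConeStruct.
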(event `self.ReceiveBeginPlay`
  (bind _defending_amount_of_ships (break `/Game/Cosmic/Blueprints/GamemodeCosmic/Structures/AmountOfShips` (`self.Defending`)))
  (bind _attacking_amount_of_ships (break `/Game/Cosmic/Blueprints/GamemodeCosmic/Structures/AmountOfShips` (`self.Attacking`)))
  (bind _defending_amount_of_ships_2 (break `/Game/Cosmic/Blueprints/GamemodeCosmic/Structures/AmountOfShips` (`self.Defending`)))
  (bind _attacking_amount_of_ships_2 (break `/Game/Cosmic/Blueprints/GamemodeCosmic/Structures/AmountOfShips` (`self.Attacking`)))
  (bind _attacking_amount_of_ships_3 (break `/Game/Cosmic/Blueprints/GamemodeCosmic/Structures/AmountOfShips` (`self.Attacking`)))
  (bind _attacking_amount_of_ships_4 (break `/Game/Cosmic/Blueprints/GamemodeCosmic/Structures/AmountOfShips` (`self.Attacking`)))
  (bind _defending_amount_of_ships_3 (break `/Game/Cosmic/Blueprints/GamemodeCosmic/Structures/AmountOfShips` (`self.Defending`)))
  (bind _defending_amount_of_ships_4 (break `/Game/Cosmic/Blueprints/GamemodeCosmic/Structures/AmountOfShips` (`self.Defending`)))
  (bind _shipstruct_amount_of_ships (break `/Game/Cosmic/Blueprints/GamemodeCosmic/Structures/AmountOfShips` (`/Game/Cosmic/Blueprints/GamemodeCosmic/Planets/BP_P_Planet.ShipStruct` (`self.Attacked Planet`))))
  (`BlueprintMapLibrary.Map_Add` _defending_amount_of_ships (`self.Color Def Player`) (`BlueprintMapLibrary.Map_Find` _shipstruct_amount_of_ships (`self.Color Def Player`)))
  (`BlueprintMapLibrary.Map_Add` _attacking_amount_of_ships_2 "Синий" 4)
  (`BlueprintMapLibrary.Map_Add` _attacking_amount_of_ships_3 "Жёлтый" 4)
  (`BlueprintMapLibrary.Map_Add` _attacking_amount_of_ships_4 "Фиолетовый" 2)
  (`BlueprintMapLibrary.Map_Add` _attacking_amount_of_ships "Зелёный" 4)
  (`BlueprintMapLibrary.Map_Add` _defending_amount_of_ships_4 "Голубой" 4)
  (`BlueprintMapLibrary.Map_Add` _defending_amount_of_ships_2 "Розовый" 4)
  (`BlueprintMapLibrary.Map_Add` _defending_amount_of_ships_3 "Жёлтый" 2)
  (`/Engine/EditorBlueprintResources/ActorMacros.Switch Has Authority`
    (:`Authority`
      (`self.UpdateShips`))))

(fn `ChangeShips`
  (params (Color :type String) (Amount :type Integer) (`Is From Warp` :type Boolean) (Where :type String))
  (bind _asbp_pc_cosmic_encounter (cast `/Game/Cosmic/Blueprints/GamemodeCosmic/BP_PC_CosmicEncounter` (`GameplayStatics.GetPlayerController` 0)))
  (`/Game/Cosmic/Blueprints/GamemodeCosmic/BP_PC_CosmicEncounter.SR_Change_Cone_Struct` _asbp_pc_cosmic_encounter self Color Amount `Is From Warp` Where))

(fn `GetPlayersOnSide`
  (params (Side :type "/Game/Cosmic/Blueprints/GamemodeCosmic/Structures/AmountOfShips Structure"))
  (returns (`Players On This Planet` :type "Array of String"))
  (locals (PlayersOnThisPlanet :type "Array of String"))
  (bind _keys (`BlueprintMapLibrary.Map_Keys` Side_Amount_Of_Ships_5_EEBC8A4C463B81C55E2E88B3A1115A37))
  (for _array_element _keys
    (if (> (`BlueprintMapLibrary.Map_Find` Side_Amount_Of_Ships_5_EEBC8A4C463B81C55E2E88B3A1115A37 _array_element) 0)
      (`KismetArrayLibrary.Array_Add` (`local.PlayersOnThisPlanet`) _array_element)))
  (return (`local.PlayersOnThisPlanet`)))

(fn `GetPositionOfShips`
  (params (`Index Of Color` :type Integer) (`Index Of Ship` :type Integer) (Max :type Integer) (`Cone Position` :type "Transform Structure") (Mode :type String) (Color :type String))
  (returns (Transform :type "Transform Structure"))
  (locals (Hypotenuse :type "Float (double-precision)" :default 400.0) (Sin :type "Float (double-precision)") (Cos :type "Float (double-precision)") (`O Small` :type "Float (double-precision)"))
  (bind _returnvalue (`self.GetTransform`))
  (bind _returnvalue_2 (`self.GetTransform`))
  (if (`KismetStringLibrary.EqualEqual_StrStr` Mode "Attacking")
    (if (`KismetStringLibrary.EqualEqual_StrStr` (`self.Color Off Player`) (`local.Color`))
      (return (`KismetMathLibrary.MakeTransform` (`KismetMathLibrary.MakeVector` (* (.x (.location _returnvalue_2)) 1.2) (* (.y (.location _returnvalue_2)) 1.2) (`KismetMathLibrary.Conv_IntToDouble` (+ (* (`local.Index Of Ship`) 8) 7))) (struct) (1.5 1.5 1.0)))
      (else
        (bind _outactors (`GameplayStatics.GetAllActorsOfClass` "/Game/Cosmic/Blueprints/GamemodeCosmic/Planets/BP_P_Planet.BP_P_Planet_C"))
        (if (== (mod (`local.Max`) 2) 0)
          (set `local.O Small` 0.1))
        (bind _returnvalue_3 (`KismetMathLibrary.Conv_IntToDouble` (- (`KismetArrayLibrary.Array_Length` _outactors) 1)))
        (bind _returnvalue_4 (* (`KismetMathLibrary.MultiplyByPi` (/ (mod (+ (* (+ (* (`KismetMathLibrary.Conv_IntToDouble` (- (/ Max 2) `Index Of Color`)) 0.2) (`local.O Small`)) (`self.Players`)) (`KismetMathLibrary.Conv_IntToDouble` (`self.Number Of Attacked Planet`))) _returnvalue_3) _returnvalue_3)) 2.0))
        (return (`KismetMathLibrary.MakeTransform` (`KismetMathLibrary.MakeVector` (* 166.0 (`KismetMathLibrary.Cos` _returnvalue_4)) (* (`KismetMathLibrary.Sin` _returnvalue_4) 166.0) (`KismetMathLibrary.Conv_IntToDouble` (+ (* `Index Of Ship` 8) 7))) (struct) (1.5 1.5 1.0)))))
    (elif (`KismetStringLibrary.EqualEqual_StrStr` (`self.Color Def Player`) (`local.Color`))
      (return (`KismetMathLibrary.MakeTransform` (0.0 0.0 1000.0) (struct) (1.5 1.5 1.0)))
      (else
        (bind _outactors_2 (`GameplayStatics.GetAllActorsOfClass` "/Game/Cosmic/Blueprints/GamemodeCosmic/Planets/BP_P_Planet.BP_P_Planet_C"))
        (if (== (mod (`local.Max`) 2) 0)
          (set `local.O Small` 0.2))
        (bind _returnvalue_5 (`KismetMathLibrary.Conv_IntToDouble` (- (`KismetArrayLibrary.Array_Length` _outactors_2) 1)))
        (bind _returnvalue_6 (* (`KismetMathLibrary.MultiplyByPi` (+ (/ (mod (+ (* (+ (* (`KismetMathLibrary.Conv_IntToDouble` (- (/ Max 2) `Index Of Color`)) 0.4) (`local.O Small`)) (`self.Players`)) (`KismetMathLibrary.Conv_IntToDouble` (`self.Number Of Attacked Planet`))) _returnvalue_5) _returnvalue_5) 0.5)) 2.0))
        (return (`KismetMathLibrary.MakeTransform` (`KismetMathLibrary.MakeVector` (+ (* 75.0 (`KismetMathLibrary.Cos` _returnvalue_6)) (* (.x (.location _returnvalue)) 2.0)) (+ (* (`KismetMathLibrary.Sin` _returnvalue_6) 75.0) (* (.y (.location _returnvalue)) 2.0)) (`KismetMathLibrary.Conv_IntToDouble` (+ (* `Index Of Ship` 8) 7))) (struct) (1.5 1.5 1.0)))))))

(fn `UpdateShips`
  (bind _attacking_amount_of_ships (break `/Game/Cosmic/Blueprints/GamemodeCosmic/Structures/AmountOfShips` (`self.Attacking`)))
  (bind _defending_amount_of_ships (break `/Game/Cosmic/Blueprints/GamemodeCosmic/Structures/AmountOfShips` (`self.Defending`)))
  (bind _attacking_amount_of_ships_2 (break `/Game/Cosmic/Blueprints/GamemodeCosmic/Structures/AmountOfShips` (`self.Attacking`)))
  (bind _players_on_this_planet (`self.GetPlayersOnSide` (`self.Defending`)))
  (bind _players_on_this_planet_2 (`self.GetPlayersOnSide` (`self.Attacking`)))
  (bind _returnvalue (> (`BlueprintMapLibrary.Map_Find` _attacking_amount_of_ships_2 (`self.Color Off Player`)) 0))
  (bind _outactors (`GameplayStatics.GetAllActorsOfClass` "/Game/Cosmic/Blueprints/GamemodeCosmic/Planets/BP_P_Ship.BP_P_Ship_C"))
  (for _array_element _outactors
    (if (== self (`self.GetOwner` _array_element))
      (`self.K2_DestroyActor` _array_element)))
  (for (_array_element_2 _array_index) _players_on_this_planet_2
    (for _index (range 1 (+ (`BlueprintMapLibrary.Map_Find` _attacking_amount_of_ships _array_element_2) 1))
      (bind _transform (`self.GetPositionOfShips` (- _array_index _returnvalue) _index (- (`KismetArrayLibrary.Array_Length` _players_on_this_planet_2) _returnvalue) (`self.GetTransform`) "Attacking" _array_element_2))
      (`|SpawnActorFromClass` "/Game/Cosmic/Blueprints/GamemodeCosmic/Planets/BP_P_Ship.BP_P_Ship_C" _transform "Undefined" "MultiplyWithRoot" self _array_element_2 null null)))
  (for (_array_element_3 _array_index_2) _players_on_this_planet
    (for _index_2 (range 1 (+ (`BlueprintMapLibrary.Map_Find` _defending_amount_of_ships _array_element_3) 1))
      (bind _transform_2 (`self.GetPositionOfShips` _array_index_2 _index_2 (`KismetArrayLibrary.Array_Length` _players_on_this_planet) (`self.GetTransform`) "Defending" _array_element_3))
      (`|SpawnActorFromClass` "/Game/Cosmic/Blueprints/GamemodeCosmic/Planets/BP_P_Ship.BP_P_Ship_C" _transform_2 "Undefined" "MultiplyWithRoot" self _array_element_3 null null))))

(fn `UserConstructionScript`)