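; Player controller for the Cosmic Encounter game mode, handling each player's UI, chat, camera turn toward the board and color selection.
; The local controller creates chat, player list, spacer and card HUD widgets, with Tab showing the list and Enter focusing chat.
; Submitted chat is relayed to every controller in PlayerArray.
; Color picks pass player by player through GameState, then a server message announces planet creation and GameMode starts spawning.
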(event `Rotate_To_Board`
  (params (Pawn :type "Pawn Object Reference"))
  (`self.SetControlRotation` self (`KismetMathLibrary.RInterpTo` (`Pawn.GetControlRotation` Pawn) (`KismetMathLibrary.FindLookAtRotation` (`self.K2_GetActorLocation` Pawn) (0.0 0.0 -100.0)) (`GameplayStatics.GetWorldDeltaSeconds`))))

(event `Key|Slash`
  (params (Key :type "Key Structure"))
  (:`Pressed`
    (bind _outactors (`GameplayStatics.GetAllActorsOfClass` "/Script/Engine.DefaultPawn"))
    (for _array_element _outactors
      (`KismetSystemLibrary.PrintString` (`KismetStringLibrary.Conv_RotatorToString` (`self.K2_GetActorRotation` _array_element))))))

(event `Key|Tab`
  (params (Key :type "Key Structure"))
  (bind _player_panel (`self.Player_Panel`))
  (:`Pressed`
    (`Widget.SetVisibility` _player_panel "Visible"))
  (:`Released`
    (`Widget.SetVisibility` _player_panel "Collapsed")))

(event `self.ReceiveBeginPlay`
  (if (`self.IsLocalPlayerController`)
    (bind _returnvalue (`|CreateWidget` "/Game/Cosmic/Blueprints/GamemodeCosmic/Widgets/BP_W_ChatWindow.BP_W_ChatWindow_C" self))
    (bind _output_get (set `self.Chat_Panel` _returnvalue))
    (`UserWidget.AddToViewport` (`self.Chat_Panel`) 0)
    (`UserWidget.AddToViewport` _output_get 0)
    (bind _returnvalue_2 (`|CreateWidget` "/Game/Cosmic/Blueprints/GamemodeCosmic/Widgets/BP_W_PlayerList.BP_W_PlayerList_C" self))
    (bind _output_get_2 (set `self.Player_Panel` _returnvalue_2))
    (`Widget.SetVisibility` _output_get_2 "Collapsed")
    (`UserWidget.AddToViewport` (`self.Player_Panel`) 0)
    (`UserWidget.AddToViewport` _output_get_2 0)
    (bind _returnvalue_3 (`|CreateWidget` "/Game/Cosmic/Blueprints/GamemodeCosmic/Widgets/BP_W_EmptySpace.BP_W_EmptySpace_C" self))
    (bind _output_get_3 (set `self.Empty_Panel` _returnvalue_3))
    (`UserWidget.AddToViewport` _output_get_3 0)
    (`UserWidget.AddToViewport` (`self.Empty_Panel`) 0)
    (bind _returnvalue_4 (`|CreateWidget` "/Game/Cosmic/Blueprints/GamemodeCosmic/Cards/BP_W_CardHUD.BP_W_CardHUD_C" self))
    (`UserWidget.AddToViewport` _returnvalue_4 0)))

(event `Key|Enter`
  (params (Key :type "Key Structure"))
  (:`Pressed`
    (bind _chat_panel (`self.Chat_Panel`)
      (:`then`
        (`Widget.SetKeyboardFocus` (`/Game/Cosmic/Blueprints/GamemodeCosmic/Widgets/BP_W_ChatWindow.ChatInput_TB` _chat_panel)))
      (:`else`))))

(event `SR_SubmitChat`
  (params (PlayerName :type Text) (Message :type Text) (PlayerColor :type "Color Structure"))
  (`KismetSystemLibrary.Delay` 0.5)
  (for _array_element (`GameStateBase.PlayerArray` (`GameplayStatics.GetGameState`))
    (bind _asbp_pc_cosmic_encounter (cast `/Game/Cosmic/Blueprints/GamemodeCosmic/BP_PC_CosmicEncounter` (`PlayerState.GetPlayerController` _array_element)))
    (`self.OC_UpdateChat` :`self` _asbp_pc_cosmic_encounter :`PlayerName` PlayerName :`Message` Message)))

(event `OC_UpdateChat`
  (params (PlayerName :type Text) (Message :type Text) (PlayerColor :type "Color Structure"))
  (bind _chat_panel (`self.Chat_Panel`)
    (:`then`
      (`/Game/Cosmic/Blueprints/GamemodeCosmic/Widgets/BP_W_ChatWindow.Update_Chat` :`self` _chat_panel :`PlayerName` PlayerName :`ChatMessage` Message))
    (:`else`)))

(event `Choose_Color`
  (params (Player :type Integer))
  (bind _returnvalue (`|CreateWidget` "/Game/Cosmic/Blueprints/GamemodeCosmic/Widgets/BP_W_ChooseColor.BP_W_ChooseColor_C" self Player))
  (`UserWidget.AddToViewport` _returnvalue 0))

(event `SR_Choosed_Color`
  (params (Player :type Integer) (Color :type String))
  (bind _returnvalue (+ Player 1))
  (bind _asbp_ps_cosmic_encounter (cast `/Game/Cosmic/Blueprints/GamemodeCosmic/BP_PS_CosmicEncounter` (`GameplayStatics.GetPlayerState` Player)))
  (`/Game/Cosmic/Blueprints/GamemodeCosmic/BP_PS_CosmicEncounter.SR_Selecting_Color` _asbp_ps_cosmic_encounter Color)
  (cast `/Game/Cosmic/Blueprints/GamemodeCosmic/BP_PS_CosmicEncounter` (`GameplayStatics.GetPlayerState` _returnvalue)
    (:`then`
      (`KismetSystemLibrary.Delay` 1.0)
      (bind _asbp_gs_cosmic_encounter (cast `/Game/Cosmic/Blueprints/GamemodeCosmic/BP_GS_CosmicEncounter` (`GameplayStatics.GetGameState`)))
      (`/Game/Cosmic/Blueprints/GamemodeCosmic/BP_GS_CosmicEncounter.SR_Choose_Color` _asbp_gs_cosmic_encounter _returnvalue Color))
    (:`CastFailed`
      (`KismetSystemLibrary.Delay` 1.0)
      (`self.SR_SubmitChat` "Сервер" "Все игроки успешно выбрали цвета! Создаю планеты...")
      (bind _asbp_gm_cosmic_encounter (cast `/Game/Cosmic/Blueprints/GamemodeCosmic/BP_GM_CosmicEncounter` (`GameplayStatics.GetGameMode`)))
      (`/Game/Cosmic/Blueprints/GamemodeCosmic/BP_GM_CosmicEncounter.Start_Spawn` _asbp_gm_cosmic_encounter))))

(fn `UserConstructionScript`)