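; Game mode for Cosmic Encounter that gathers players and starts the color draft.
; It reads the expected player count from the options string and tracks controllers on login and logout, announcing both in Russian chat.
; Each change triggers a delayed GameState player-list refresh and, when the count matches, starts the draft with the first controller.
; The draft prompts that player to choose a color; its trailing loop over all controllers only casts.
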(event `Update_PlayerList`
  (`KismetSystemLibrary.Delay` 0.3)
  (bind _asbp_gs_cosmic_encounter (cast `/Game/Cosmic/Blueprints/GamemodeCosmic/BP_GS_CosmicEncounter` (`GameplayStatics.GetGameState`)))
  (`/Game/Cosmic/Blueprints/GamemodeCosmic/BP_GS_CosmicEncounter.Update_PlayerList` _asbp_gs_cosmic_encounter))

(event `self.ReceiveBeginPlay`
  (set `self.Players` (`KismetMathLibrary.Conv_IntToByte` (`KismetStringLibrary.Conv_StringToInt` (`GameplayStatics.ParseOption` (`self.OptionsString`) "Players")))))

(event `self.K2_PostLogin`
  (params (NewPlayer :type "PlayerController Object Reference"))
  (bind _asbp_pc_cosmic_encounter (cast `/Game/Cosmic/Blueprints/GamemodeCosmic/BP_PC_CosmicEncounter` NewPlayer))
  (`/Game/Cosmic/Blueprints/GamemodeCosmic/BP_PC_CosmicEncounter.SR_SubmitChat` :`self` _asbp_pc_cosmic_encounter :`PlayerName` (`KismetTextLibrary.Conv_StringToText` (`PlayerState.GetPlayerName` (`Controller.PlayerState` NewPlayer))) :`Message` " подключился к игре.")
  (`KismetArrayLibrary.Array_Add` (`self.All PCs`) _asbp_pc_cosmic_encounter)
  (`self.Update_PlayerList` :!label _label)
  (if (== (`KismetArrayLibrary.Array_Length` (`self.All PCs`)) (`self.Players`))
    (`self.Start_Color_Draft` 0)))

(event `self.K2_OnLogout`
  (params (ExitingController :type "Controller Object Reference"))
  (bind _asbp_pc_cosmic_encounter (cast `/Game/Cosmic/Blueprints/GamemodeCosmic/BP_PC_CosmicEncounter` ExitingController))
  (`/Game/Cosmic/Blueprints/GamemodeCosmic/BP_PC_CosmicEncounter.SR_SubmitChat` :`self` _asbp_pc_cosmic_encounter :`PlayerName` (`KismetTextLibrary.Conv_StringToText` (`PlayerState.GetPlayerName` (`Controller.PlayerState` ExitingController))) :`Message` "вышел из игры.")
  (`KismetArrayLibrary.Array_RemoveItem` (`self.All PCs`) _asbp_pc_cosmic_encounter)
  (goto _label))

(event `Start_Color_Draft`
  (params (`Player Number` :type Integer))
  (bind _asbp_pc_cosmic_encounter (cast `/Game/Cosmic/Blueprints/GamemodeCosmic/BP_PC_CosmicEncounter` (`PlayerState.GetPlayerController` (`Controller.PlayerState` (`|GetArrayItem` (`self.All PCs`) `Player Number`)))))
  (`/Game/Cosmic/Blueprints/GamemodeCosmic/BP_PC_CosmicEncounter.Choose_Color` _asbp_pc_cosmic_encounter `Player Number`)
  (`/Game/Cosmic/Blueprints/GamemodeCosmic/BP_PC_CosmicEncounter.SR_SubmitChat` :`self` _asbp_pc_cosmic_encounter :`PlayerName` "Сервер" :`Message` "Начался выбор цвета.")
  (for _array_element (`self.All PCs`)
    (cast `/Game/Cosmic/Blueprints/GamemodeCosmic/BP_PC_CosmicEncounter` (`PlayerState.GetPlayerController` (`Controller.PlayerState` _array_element)))))

(fn `UserConstructionScript`)