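; Player state for the Cosmic Encounter game mode, tracking one player's hand, card count, color and far colony count.
; SR_ events add cards and set the color, also copying it to the player controller and game state.
; OC_ events update the card hand widget and show alliance prompts offering attack, defense or pass according to invitations.
; OnRep functions for color, card count and colonies refresh every player list widget.
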(event `OC_AddCard`
  (params (CardInfo :type "/Game/Cosmic/Blueprints/GamemodeCosmic/Cards/BPS_CardInfo Structure"))
  (bind _foundwidgets (`WidgetBlueprintLibrary.GetAllWidgetsOfClass` "/Game/Cosmic/Blueprints/GamemodeCosmic/Cards/BP_W_CardHand.BP_W_CardHand_C" false))
  (message `/Game/Cosmic/Blueprints/GamemodeCosmic/Cards/BPI_AddCard.AddCard` (`|GetArrayItem` _foundwidgets) CardInfo))

(event `SR_AddCard`
  (params (Card :type "/Game/Cosmic/Blueprints/GamemodeCosmic/Cards/BPS_CardInfo Structure"))
  (bind _playerhand_cards (break `/Game/Cosmic/Blueprints/GamemodeCosmic/Structures/CardsInHand` (`self.PlayerHand`)))
  (set `self.PlayerCards` (+ (`self.PlayerCards`) 1))
  (`self.OC_AddCard` Card)
  (`KismetArrayLibrary.Array_Add` _playerhand_cards Card))

(event `SR_Selecting_Color`
  (params (Color :type String))
  (bind _output_get (set `self.PlayerColorStr` Color))
  (set `self.PlayerColorClr` (`BlueprintMapLibrary.Map_Find` (`self.ArrayOfColors`) _output_get))
  (bind _asbp_pc_cosmic_encounter (cast `/Game/Cosmic/Blueprints/GamemodeCosmic/BP_PC_CosmicEncounter` (`self.GetPlayerController` self)))
  (set `/Game/Cosmic/Blueprints/GamemodeCosmic/BP_PC_CosmicEncounter.Color` Color _asbp_pc_cosmic_encounter)
  (bind _asbp_gs_cosmic_encounter (cast `/Game/Cosmic/Blueprints/GamemodeCosmic/BP_GS_CosmicEncounter` (`GameplayStatics.GetGameState`)))
  (`BlueprintMapLibrary.Map_Add` (`/Game/Cosmic/Blueprints/GamemodeCosmic/BP_GS_CosmicEncounter.PlayerState_Color` _asbp_gs_cosmic_encounter) self Color))

(event `OC_Alliances`
  (params (`Offense Invitation` :type Boolean) (`Defense Invitation` :type Boolean))
  (`KismetSystemLibrary.PrintString` (`KismetStringLibrary.Concat_StrStr` (`KismetStringLibrary.Conv_BoolToString` `Offense Invitation`) (`KismetStringLibrary.Conv_BoolToString` `Defense Invitation`)))
  (if (and (== `Offense Invitation` true) (== `Defense Invitation` true))
    (bind _returnvalue (`|CreateWidget` "/Game/Cosmic/Blueprints/GamemodeCosmic/Widgets/BP_W_MessageForPlayer.BP_W_MessageForPlayer_C" (`self.GetPlayerController`) "Будете ли вы участвовать в контакте?" true "За атаку" "За защиту" "Пас"))
    (`UserWidget.AddToViewport` _returnvalue 0)
    (elif (and (== `Offense Invitation` true) (== `Defense Invitation` false))
      (bind _returnvalue_2 (`|CreateWidget` "/Game/Cosmic/Blueprints/GamemodeCosmic/Widgets/BP_W_MessageForPlayer.BP_W_MessageForPlayer_C" (`self.GetPlayerController`) "Будете ли вы участвовать в контакте?" true "За атаку" "" "Пас"))
      (`UserWidget.AddToViewport` _returnvalue_2 0)
      (else
        (bind _returnvalue_3 (`|CreateWidget` "/Game/Cosmic/Blueprints/GamemodeCosmic/Widgets/BP_W_MessageForPlayer.BP_W_MessageForPlayer_C" (`self.GetPlayerController`) "Будете ли вы участвовать в контакте?" true "" "За защиту" "Пас"))
        (`UserWidget.AddToViewport` _returnvalue_3 0)))))

(fn `ChangeFarColonies`
  (params (Amount :type Integer))
  (if (!= Amount 0)
    (set `self.PlayerFarColonies` (+ Amount (`self.PlayerFarColonies`)))
    (else
      (set `self.PlayerFarColonies` 0))))

(fn `OnRep_PlayerCards`
  (bind _foundwidgets (`WidgetBlueprintLibrary.GetAllWidgetsOfClass` "/Game/Cosmic/Blueprints/GamemodeCosmic/Widgets/BP_W_PlayerList.BP_W_PlayerList_C" false))
  (for _array_element _foundwidgets
    (`/Game/Cosmic/Blueprints/GamemodeCosmic/Widgets/BP_W_PlayerList.Update_Widget` _array_element)))

(fn `OnRep_PlayerColorStr`
  (bind _foundwidgets (`WidgetBlueprintLibrary.GetAllWidgetsOfClass` "/Game/Cosmic/Blueprints/GamemodeCosmic/Widgets/BP_W_PlayerList.BP_W_PlayerList_C" false))
  (for _array_element _foundwidgets
    (`/Game/Cosmic/Blueprints/GamemodeCosmic/Widgets/BP_W_PlayerList.Update_Widget` _array_element)))

(fn `OnRep_PlayerFarColonies`
  (bind _foundwidgets (`WidgetBlueprintLibrary.GetAllWidgetsOfClass` "/Game/Cosmic/Blueprints/GamemodeCosmic/Widgets/BP_W_PlayerList.BP_W_PlayerList_C" false))
  (for _array_element _foundwidgets
    (`/Game/Cosmic/Blueprints/GamemodeCosmic/Widgets/BP_W_PlayerList.Update_Widget` _array_element)))

(fn `UserConstructionScript`)