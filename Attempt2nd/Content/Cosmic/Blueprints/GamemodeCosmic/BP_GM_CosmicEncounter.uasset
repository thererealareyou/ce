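; Game mode for Cosmic Encounter that tracks connected players and triggers player list updates.
; On BeginPlay it reads the expected player count from the "Players" option in the options string.
; Login and logout add or remove Cosmic Encounter player controllers in AllPCs, then request a list update.
; The update event waits briefly before telling the game state to refresh its player list.
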(event `self.ReceiveBeginPlay`
  (set `self.Players` (`KismetMathLibrary.Conv_IntToByte` (`KismetStringLibrary.Conv_StringToInt` (`GameplayStatics.ParseOption` (`self.OptionsString`) "Players")))))

(event `Update_PlayerList`
  (`KismetSystemLibrary.Delay` 0.3)
  (bind _asbp_gs_cosmic_encounter (cast `/Game/Cosmic/Blueprints/GamemodeCosmic/BP_GS_CosmicEncounter` (`GameplayStatics.GetGameState`)))
  (`/Game/Cosmic/Blueprints/GamemodeCosmic/BP_GS_CosmicEncounter.Update_PlayerList` _asbp_gs_cosmic_encounter))

(event `self.K2_PostLogin`
  (params (NewPlayer :type "PlayerController Object Reference"))
  (bind _asbp_pc_cosmic_encounter (cast `/Game/Cosmic/Blueprints/GamemodeCosmic/BP_PC_CosmicEncounter` NewPlayer))
  (`KismetArrayLibrary.Array_Add` (`self.All PCs`) _asbp_pc_cosmic_encounter)
  (`self.Update_PlayerList` :!label _label))

(event `self.K2_OnLogout`
  (params (ExitingController :type "Controller Object Reference"))
  (bind _asbp_pc_cosmic_encounter (cast `/Game/Cosmic/Blueprints/GamemodeCosmic/BP_PC_CosmicEncounter` ExitingController))
  (`KismetArrayLibrary.Array_RemoveItem` (`self.All PCs`) _asbp_pc_cosmic_encounter)
  (goto _label))

(fn `UserConstructionScript`)