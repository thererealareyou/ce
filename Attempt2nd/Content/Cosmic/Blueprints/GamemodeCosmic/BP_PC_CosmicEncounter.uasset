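; Player controller for the Cosmic Encounter game mode, handling local UI, text chat and turn state.
; On BeginPlay the local controller creates chat, player list and empty-space widgets; holding Tab shows the list and Enter focuses chat input.
; SR_SubmitChat relays messages through every controller in PlayerArray to OC_UpdateChat and its chat widget, without forwarding PlayerColor.
; SetMyTurn stores the turn value and broadcasts the change through a dispatcher.
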(event `Key|Tab`
  (params (Key :type "Key Structure"))
  (bind _player_panel (`self.Player_Panel`))
  (:`Pressed`
    (`Widget.SetVisibility` _player_panel "Visible"))
  (:`Released`
    (`Widget.SetVisibility` _player_panel "Collapsed")))

(event `self.ReceiveBeginPlay`
  (bind _player_panel (`self.Player_Panel`))
  (if (`self.IsLocalPlayerController`)
    (bind _returnvalue (`|CreateWidget` "/Game/Cosmic/Blueprints/GamemodeCosmic/Widgets/BP_W_ChatWindow.BP_W_ChatWindow_C" self))
    (bind _output_get (set `self.Chat_Panel` _returnvalue))
    (`UserWidget.AddToViewport` (`self.Chat_Panel`) 0)
    (`UserWidget.AddToViewport` _output_get 0)
    (bind _returnvalue_2 (`|CreateWidget` "/Game/Cosmic/Blueprints/GamemodeCosmic/Widgets/BP_W_PlayerList.BP_W_PlayerList_C" self))
    (bind _output_get_2 (set `self.Player_Panel` _returnvalue_2))
    (`Widget.SetVisibility` _player_panel "Collapsed")
    (`UserWidget.AddToViewport` _player_panel 0)
    (`UserWidget.AddToViewport` _output_get_2 0)
    (bind _returnvalue_3 (`|CreateWidget` "/Game/Cosmic/Blueprints/GamemodeCosmic/Widgets/BP_W_EmptySpace.BP_W_EmptySpace_C" self))
    (bind _output_get_3 (set `self.Empty_Panel` _returnvalue_3))
    (`UserWidget.AddToViewport` _output_get_3 0)
    (`UserWidget.AddToViewport` (`self.Empty_Panel`) 0)))

(event `Key|Enter`
  (params (Key :type "Key Structure"))
  (:`Pressed`
    (bind _chat_panel (`self.Chat_Panel`)
      (:`then`
        (`Widget.SetKeyboardFocus` (`/Game/Cosmic/Blueprints/GamemodeCosmic/Widgets/BP_W_ChatWindow.ChatInput_TB` _chat_panel)))
      (:`else`))))

(event `SR_SubmitChat`
  (params (PlayerName :type Text) (Message :type Text) (PlayerColor :type "Color Structure"))
  (for _array_element (`GameStateBase.PlayerArray` (`GameplayStatics.GetGameState`))
    (bind _asbp_pc_cosmic_encounter (cast `/Game/Cosmic/Blueprints/GamemodeCosmic/BP_PC_CosmicEncounter` (`PlayerState.GetPlayerController` _array_element)))
    (`self.OC_UpdateChat` :`self` _asbp_pc_cosmic_encounter :`PlayerName` PlayerName :`Message` Message)))

(event `OC_UpdateChat`
  (params (PlayerName :type Text) (Message :type Text) (PlayerColor :type "Color Structure"))
  (bind _chat_panel (`self.Chat_Panel`)
    (:`then`
      (`/Game/Cosmic/Blueprints/GamemodeCosmic/Widgets/BP_W_ChatWindow.Update_Chat` :`self` _chat_panel :`PlayerName` PlayerName :`ChatMessage` Message))
    (:`else`)))

(fn `SetMyTurn`
  (params (Turn :type Boolean))
  (bind _output_get (set `self.Set_My_Turn` Turn))
  (`self.OnMyTurnChanges` _output_get))

(fn `UserConstructionScript`)