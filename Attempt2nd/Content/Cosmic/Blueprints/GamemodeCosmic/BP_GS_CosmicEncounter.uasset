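; Game state for the Cosmic Encounter mode that tracks joined players and signals the color draft once the lobby is full.
; BeginPlay reads the expected player count from the game mode, and Update_PlayerList copies PlayerArray into AllPlayerStates, firing the draft-color event on the server when counts match.
; The AllPlayerStates RepNotify refreshes player-list widgets, updating every empty-space widget inside that loop.
; The MC_Draft_Color event body is empty here.
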(event `self.ReceiveBeginPlay`
  (bind _asbp_gm_cosmic_encounter (cast `/Game/Cosmic/Blueprints/GamemodeCosmic/BP_GM_CosmicEncounter` (`GameplayStatics.GetGameMode`)))
  (set `self.Players` (`/Game/Cosmic/Blueprints/GamemodeCosmic/BP_GM_CosmicEncounter.Players` _asbp_gm_cosmic_encounter)))

(event `Update_PlayerList`
  (bind _output_get (set `self.All Player States` (`self.PlayerArray`)))
  (if (== (`KismetArrayLibrary.Array_Length` _output_get) (`self.Players`))
    (if (`KismetSystemLibrary.IsServer`)
      (`self.MC_Draft_Color`))))

(event `MC_Draft_Color`)

(fn `OnRep_All Player States`
  (bind _foundwidgets (`WidgetBlueprintLibrary.GetAllWidgetsOfClass` "/Game/Cosmic/Blueprints/GamemodeCosmic/Widgets/BP_W_PlayerList.BP_W_PlayerList_C" false))
  (for _array_element _foundwidgets
    (`/Game/Cosmic/Blueprints/GamemodeCosmic/Widgets/BP_W_PlayerList.Update_Widget` _array_element)
    (bind _foundwidgets_2 (`WidgetBlueprintLibrary.GetAllWidgetsOfClass` "/Game/Cosmic/Blueprints/GamemodeCosmic/Widgets/BP_W_EmptySpace.BP_W_EmptySpace_C" false))
    (for _array_element_2 _foundwidgets_2
      (`/Game/Cosmic/Blueprints/GamemodeCosmic/Widgets/BP_W_EmptySpace.Update Widget` _array_element_2))))

(fn `UserConstructionScript`)